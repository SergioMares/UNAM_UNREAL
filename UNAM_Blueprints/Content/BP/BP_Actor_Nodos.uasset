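; Debug-style actor that prints a fixed message on screen in a randomly generated text color.
; Every Tick, RandomColor builds a color with random RGBA channels and passes it to ChangeColorText.
; ChangeColorText waits on a Delay, stores the color only while the ChangeColor flag is set, clears that flag, then prints the string.
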(event `self.ReceiveTick`
  (params (DeltaSeconds :type "Float (single-precision)"))
  (bind _color (`self.RandomColor`))
  (`self.ChangeColorText` _color))

(fn `RandomColor`
  (returns (Color :type "Color Structure"))
  (return (make `Color` (`KismetMathLibrary.Conv_IntToByte` (`KismetMathLibrary.RandomIntegerInRange` 0 255)) (`KismetMathLibrary.Conv_IntToByte` (`KismetMathLibrary.RandomIntegerInRange` 0 255)) (`KismetMathLibrary.Conv_IntToByte` (`KismetMathLibrary.RandomIntegerInRange` 0 255)) (`KismetMathLibrary.Conv_IntToByte` (`KismetMathLibrary.RandomIntegerInRange` 0 255)))))

(fn `UserConstructionScript`)